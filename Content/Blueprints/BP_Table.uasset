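; BP_Table is a table actor that erodes away and destroys itself once the first-person character touches its box trigger.
; The first overlap creates a dynamic instance of MI_DisappearingBench, applies it to the table mesh and starts a one-shot countdown from ErosionDuration.
; Tick drives the material's MaskValue from the normalized remaining time, then destroys the actor when the countdown reaches zero.
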(event `self.Box.OnComponentBeginOverlap`
  (params (OverlappedComponent :type "PrimitiveComponent Object Reference") (OtherActor :type "Actor Object Reference") (OtherComp :type "PrimitiveComponent Object Reference") (OtherBodyIndex :type Integer) (bFromSweep :type Boolean) (SweepResult :type "HitResult Structure (by ref)"))
  (bind _asbp_first_person_character (cast `/Game/FirstPerson/Blueprints/BP_FirstPersonCharacter` OtherActor))
  (`/Engine/EditorBlueprintResources/StandardMacros.IsValid` _asbp_first_person_character
    (:`Is Valid`
      (if (not (`self.bEroding`))
        (set `self.bEroding` true)
        (set `self.ErosionValue` (`self.ErosionDuration`))
        (bind _returnvalue (`KismetMaterialLibrary.CreateDynamicMaterialInstance` "/Game/Materials/DisappearingMat_Exam/MI_DisappearingBench.MI_DisappearingBench"))
        (bind _output_get (set `self.DynamicMat` _returnvalue))
        (`MaterialInstanceDynamic.SetScalarParameterValue` _output_get "MaskValue" (`self.ErosionValue`))
        (`PrimitiveComponent.SetMaterial` (`self.SM_Table`) 0 (`self.DynamicMat`))))))

(event `self.ReceiveTick`
  (params (DeltaSeconds :type "Float (single-precision)"))
  (if (`self.bEroding`)
    (bind _output_get (set `self.ErosionValue` (- (`self.ErosionValue`) DeltaSeconds)))
    (`MaterialInstanceDynamic.SetScalarParameterValue` (`self.DynamicMat`) "MaskValue" (/ _output_get (`self.ErosionDuration`)))
    (if (<= (`self.ErosionValue`) 0.0)
      (`self.K2_DestroyActor`))))

(fn `UserConstructionScript`)